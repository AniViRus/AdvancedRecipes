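; BP_UnlockAdvancedRecipe is a schematic unlock Blueprint, named for advanced recipes, that supplies reward display, cost and unlock data.
; Its stinger widget data, trading post reward widget and cost functions simply forward to the parent implementations.
; GetUnlockDataStruct returns the UnmutableDataStructs variable directly, with no parent call or added logic.
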(fn `GetCost`
  (params (UnlockStructIndex :type Integer))
  (returns (cost :type "Array of ItemAmount Structure"))
  (bind _cost (`parent.GetCost` UnlockStructIndex))
  (return _cost))

(fn `GetStingerWidgetRewardData`
  (returns (StingerRewardTypes :type "Set of FGStingerWidgetRewardData Class Reference"))
  (bind _stingerrewardtypes (`parent.GetStingerWidgetRewardData`))
  (return _stingerrewardtypes))

(fn `GetUnlockDataStruct`
  (returns (UnlockDataStruct :type "Array of /Game/FactoryGame/Unlocks/FUnlockDataStruct Structure"))
  (return (`self.UnmutableDataStructs`)))

(fn `GetUnlockRewardWidgets`
  (params (OwningPlayer :type "PlayerController Object Reference") (SchematicClass :type "FGSchematic Class Reference") (TradingPostWidget :type "UserWidget Object Reference"))
  (returns (Widgets :type "Array of UserWidget Object Reference"))
  (bind _widgets (`parent.GetUnlockRewardWidgets` OwningPlayer SchematicClass TradingPostWidget))
  (return _widgets))